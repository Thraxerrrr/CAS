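; Base attachable lantern actor that a player character carries and toggles with Shift+L.
; A looping timer on non-dedicated instances checks whether the local player controls the parent BasePlayerChar, then enables input and stops.
; The key press passes the opposite lantern state to ToggleLights on the parent's BP_CAS_player_comp.
; The replicated IsLanternOn state's OnRep switches the flame effect and light visibility.
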(event `self.ReceiveBeginPlay`
  (bind _returnvalue (`KismetSystemLibrary.K2_SetTimerDelegate` (delegate `CustomEvent_0`) 5.0 true)))

(event `CustomEvent_0`
  (if (and (not (`KismetSystemLibrary.IsDedicatedServer`)) (== (`GameplayStatics.GetPlayerController` 0) (`Pawn.GetController` (cast `/Game/Characters/BasePlayerChar` (`self.GetAttachParentActor`) :!pure true))))
    (`self.EnableInput` (`GameplayStatics.GetPlayerController` 0))
    (`KismetSystemLibrary.K2_ClearAndInvalidateTimerHandle` (stale `self.ReceiveBeginPlay` _returnvalue))))

(event `Key|LeftShift`
  (params (Key :type "Key Structure" :default "AnyKey"))
  (:`Pressed`
    (set `self.isShiftDown` true :!label _label))
  (:`Released`
    (set `self.isShiftDown` false :!label _label_2)))

(event `Key|RightShift`
  (params (Key :type "Key Structure" :default "AnyKey"))
  (:`Pressed`
    (goto _label))
  (:`Released`
    (goto _label_2)))

(event `Key|L`
  (params (Key :type "Key Structure" :default "AnyKey"))
  (:`Pressed`
    (if (`self.isShiftDown`)
      (`/Game/Mods/CAS/inventory/BP_CAS_player_comp.ToggleLights` (`self.GetComponentByClass` (cast `/Game/Characters/BasePlayerChar` (`self.GetAttachParentActor`) :!pure true) "/Game/Mods/CAS/inventory/BP_CAS_player_comp.BP_CAS_player_comp_C") (not (`self.isLanternOn`))))))

(fn `OnRep_isLanternOn`
  (`ActorComponent.SetActive` (`self.LanternFlame`) (`self.isLanternOn`) false)
  (`SceneComponent.SetVisibility` (`self.Light`) (`self.isLanternOn`) false))

(fn `UserConstructionScript`
  (`parent.UserConstructionScript`))