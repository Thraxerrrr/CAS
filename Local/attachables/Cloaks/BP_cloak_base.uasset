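; Base cloak attachable Blueprint whose look is customized by a replicated blend color or a texture URL.
; Both OnRep handlers call UpdateCloak, which checks the current material's parameters to decide which customization applies.
; Color-capable cloaks get a tinted dynamic leather material.
; Texture-capable cloaks get a dynamic base cloak material showing the image downloaded at runtime, or the unmodified material when the URL is empty.
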(event `UpdateCloak`
  (bind _textureurl (`self.textureURL`))
  (bind _skeletalmeshcomp (`self.SkeletalMeshComp`))
  (bind _returnvalue (`PrimitiveComponent.GetMaterial` (`self.SkeletalMeshComp`) 0))
  (`|ExecutionSequence`
    (:`then_0`
      (bind _returnvalue_2 (`EnvironmentFunctionLibrary.DoesMaterialHaveVectorParameter` _returnvalue "BlendColor"))
      (if _returnvalue_2
        (bind _returnvalue_3 (`KismetMaterialLibrary.CreateDynamicMaterialInstance` "/Game/Mods/CAS/attachables/Cloaks/textures/M_leather_cloak.M_leather_cloak"))
        (`MaterialInstanceDynamic.SetVectorParameterValue` _returnvalue_3 "BlendColor" (`self.blendColor`))
        (`PrimitiveComponent.SetMaterial` (`self.SkeletalMeshComp`) 0 _returnvalue_3)))
    (:`then_1`
      (bind _returnvalue_4 (`EnvironmentFunctionLibrary.DoesMaterialHaveTextureParameter` _returnvalue "CloakTextureParam"))
      (if _returnvalue_4
        (if (> (`KismetStringLibrary.Len` _textureurl) 0)
          (bind _texture (`AsyncTaskDownloadImage.DownloadImage` _textureurl)
            (:`OnSuccess`
              (bind _returnvalue_5 (`KismetMaterialLibrary.CreateDynamicMaterialInstance` "/Game/Mods/CAS/attachables/Cloaks/textures/M_cloak_base.M_cloak_base"))
              (`MaterialInstanceDynamic.SetTextureParameterValue` _returnvalue_5 "CloakTextureParam" _texture)
              (`PrimitiveComponent.SetMaterial` _skeletalmeshcomp 0 _returnvalue_5)))
          (else
            (bind _returnvalue_6 (`KismetMaterialLibrary.CreateDynamicMaterialInstance` "/Game/Mods/CAS/attachables/Cloaks/textures/M_cloak_base.M_cloak_base"))
            (`PrimitiveComponent.SetMaterial` _skeletalmeshcomp 0 _returnvalue_6)))))))

(fn `OnRep_blendColor`
  (`self.UpdateCloak`))

(fn `OnRep_textureURL`
  (`self.UpdateCloak`))

(fn `UserConstructionScript`
  (`parent.UserConstructionScript`))