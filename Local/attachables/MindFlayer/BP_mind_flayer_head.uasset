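; Mind flayer head attachable that hides the head and hair of the actor it is attached to.
; On configure, it runs the parent setup, then loops through the attach parent's skeletal mesh components.
; Components whose mesh asset name contains "hair" or "head", ignoring case, have their visibility toggled without propagating to children.
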(event `self.configureAttachable`
  (`parent.configureAttachable`)
  (for _array_element (`self.K2_GetComponentsByClass` (`self.GetAttachParentActor`) "/Script/Engine.SkeletalMeshComponent")
    (bind _returnvalue (`KismetSystemLibrary.GetObjectName` (`SkinnedMeshComponent.SkeletalMesh` _array_element)))
    (if (or (`KismetStringLibrary.MatchesWildcard` _returnvalue "*hair*") (`KismetStringLibrary.MatchesWildcard` _returnvalue "*head*"))
      (`SceneComponent.ToggleVisibility` _array_element false))))

(fn `UserConstructionScript`
  (`parent.UserConstructionScript`))