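; BP_attaching_actor is an attachable actor that displays a skeletal or static mesh, such as gear on a BaseBPChar character.
; RepNotify functions on the two mesh variables apply each new mesh to its component.
; Skeletal meshes then follow the parent character's Mesh pose through SetMasterPoseComponent.
; Meshes with "bow" in their name skip that pose link, a workaround marked TODO.
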(fn `OnRep_SkeletalMesh`
  (`SkinnedMeshComponent.SetSkinnedAssetAndUpdate` (`self.SkeletalMeshComp`) (`self.SkeletalMesh`) true)
  (if (not (`KismetStringLibrary.Contains` (`KismetSystemLibrary.GetDisplayName` (`self.SkeletalMesh`)) "bow"))
    (bind _asbase_bpchar (cast `/Game/Characters/BaseBPChar` (`self.GetAttachParentActor`)))
    (`SkinnedMeshComponent.SetLeaderPoseComponent` (`self.SkeletalMeshComp`) (`Character.Mesh` _asbase_bpchar))))

(fn `OnRep_StaticMesh`
  (`StaticMeshComponent.SetStaticMesh` (`self.StaticMeshComp`) (`self.StaticMesh`)))

(fn `UserConstructionScript`)