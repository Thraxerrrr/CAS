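; Command Blueprint that registers a custom runtime transform for an item on the CAS_ModController.
; DoCommand takes a key, a location string and a rotation string, parsing both strings as comma-separated X,Y,Z through ParseVectorString.
; It maps rotation X/Y/Z to roll/pitch/yaw, fixes scale at one, and adds the transform to RuntimeItemTransforms on the first controller found, without a validity check.
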(event `self.DoCommand`
  (params (Parameters :type "Array of String (by ref)") (CallingPlayerController :type "ConanPlayerController Object Reference") (World :type "World Object Reference"))
  (bind _outactors (`GameplayStatics.GetAllActorsOfClass` "/Game/Mods/CAS/CAS_ModController.CAS_ModController_C"))
  (`BlueprintMapLibrary.Map_Add` (`/Game/Mods/CAS/CAS_ModController.runtimeItemTransforms` (`KismetArrayLibrary.Array_Get` _outactors)) (`KismetArrayLibrary.Array_Get` Parameters) (`KismetMathLibrary.MakeTransform` (`self.ParseVectorString` (`KismetArrayLibrary.Array_Get` Parameters 1)) (`KismetMathLibrary.MakeRotator` (.x (`self.ParseVectorString` (`KismetArrayLibrary.Array_Get` Parameters 2))) (.y (`self.ParseVectorString` (`KismetArrayLibrary.Array_Get` Parameters 2))) (.z (`self.ParseVectorString` (`KismetArrayLibrary.Array_Get` Parameters 2)))))))

(fn `UserConstructionScript`)