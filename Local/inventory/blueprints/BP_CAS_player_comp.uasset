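; Character component for the CAS slot system, displaying slotted items as attached actors on players and applying their buffs.
; Equip and unequip hand off to the server, which maintains CAS.Inventory and tagged actors; pouch slots depend on belt capacity.
; BeginPlay waits for replication, re-equips saved items, hides them while normally equipped, and hooks CAS buttons into player and thrall inventory screens.
; Skeletal meshes follow the character's master pose, using a delayed RPC engine-bug workaround.
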(event `EventItemAdded`
  (params (index :type Integer) (item :type "GameItem Object Reference") (srcInventory :type "ItemInventory Object Reference") (srcIndex :type Integer))
  ;[1 1 1] Initialize variables, bind event handlers
  (`self.CAS.ToggleItemVisible` item))

(event `EventItemRemoved`
  (params (index :type Integer) (item :type "GameItem Object Reference") (dstInventory :type "ItemInventory Object Reference") (dstIndex :type Integer))
  ;[1 1 1] Initialize variables, bind event handlers
  (`self.CAS.ToggleItemVisible` item true))

(event `self.ReceiveBeginPlay`
  (bind _returnvalue (`KismetArrayLibrary.Array_Length` (`self.CAS.Inventory`)))
  (`KismetSystemLibrary.Delay` 3.0) ; Give some time before we can assume replication is in place
  (`|ExecutionSequence`
    (:`then_0`
      ;[1 1 1] Initialize variables, bind event handlers
      (bind _asbase_bpchar (cast `/Game/Characters/BaseBPChar` (`self.GetOwner`)))
      (bind _output_get (set `self.ParentCharacter` _asbase_bpchar))
      (bind _inventory (`/Game/Characters/BaseBPChar.GetEquipmentInventory` _output_get))
      (add `ItemInventory.SignalItemAdded` _inventory (delegate `EventItemAdded`))
      (add `ItemInventory.SignalItemRemoved` _inventory (delegate `EventItemRemoved`)))
    (:`then_1`
      ;[1 1 1] Re-equip all saved CAS items
      (if (> _returnvalue 0)
        (for _index (range _returnvalue)
          (bind _item (`KismetArrayLibrary.Array_Get` (`self.CAS.Inventory`) _index))
          (bind _item_2 (`/Game/Mods/CAS/inventory/blueprints/BP_CAS_inventory_functions.resolveCASItem` _item (`self.ParentCharacter`)))
          (`self.CAS.TryEquipItem` _item_2 (`.SlotName_2_8DC5705C4B2832C95D9D0A8F1CA76B34` (break `/Game/Mods/CAS/inventory/blueprints/CASInventoryItem` _item))))))
    (:`then_2`
      (`/Game/Systems/BP_MacroGlobal.IsValid+Branch` (`/Game/Characters/FuncomFunctionLibrary.GetControllerFromActor` (`self.ParentCharacter`)) (not (`KismetSystemLibrary.IsDedicatedServer`))
        (:`True`
          (`|ExecutionSequence`
            (:`then_0`
              ;[1 1 1] Hook a CAS button into the player's Inventory screen
              (bind _returnvalue_2 (`GUIModuleController.GetModule` (`GUIModuleController.GetGUIModuleController`) "CharacterInventory"))
              (add `GUIModule.SignalActivated` _returnvalue_2 (delegate `OnInventoryActivated`)))
            (:`then_1`
              ;[1 1 1] Hook a CAS button into the thrall Inventory screen
              (bind _returnvalue_3 (`GUIModuleController.GetModule` (`GUIModuleController.GetGUIModuleController`) "CraftingGUI"))
              (add `GUIModule.SignalActivated` _returnvalue_3 (delegate `OnThrallInvActivated`)))))))))

(event `EventTryEquipItem`
  (params (SlotName :type String) (ItemID :type String))
  (bind _casitem (`/Game/Mods/CAS/inventory/blueprints/BP_CAS_inventory_functions.createCASItem` SlotName ItemID))
  (bind _item (`/Game/Mods/CAS/inventory/blueprints/BP_CAS_inventory_functions.resolveCASItem` _casitem (`self.ParentCharacter`)))
  (`self.CAS.TryEquipItem` _item SlotName))

(event `OnInventoryActivated`
  (params (module :type "GUIModule Object Reference") (isActive :type Boolean))
  ;[1 1 1] Hook a CAS button into the player's Inventory screen
  (if isActive
    (`self.UpdateInteractionTargetCharacter` true
      (:`execOut`
        (`KismetSystemLibrary.Delay` 0.5) ; Give the widgets some time to spawn
        (`|ExecutionSequence`
          (:`then_0`
            (bind _foundwidgets (`WidgetBlueprintLibrary.GetAllWidgetsOfClass` "/Script/ConanSandbox.UICharacterDisplay" false))
            (for _array_element _foundwidgets
              (`self.MakeCASInventoryButton` (`Widget.GetParent` (`Widget.GetParent` _array_element))))))))))

(event `EventTryUnequipItem`
  (params (SlotName :type String))
  (`self.CAS.TryUnequipItem` SlotName))

(event `EventUpdateSkeletalMesh`
  (params (TargetComponent :type "SkinnedMeshComponent Object Reference") (SkeletalMesh :type "SkeletalMesh Object Reference"))
  ;[1 1 1] Workaround, see https://issues.unrealengine.com/issue/UE-76862
  (`KismetSystemLibrary.Delay` 1.0)
  (`self.EventRPCUpdateSkeletalMesh` TargetComponent SkeletalMesh))

(event `OnThrallInvActivated`
  (params (module :type "GUIModule Object Reference") (isActive :type Boolean))
  ;[1 1 1] Hook a CAS button into the thrall Inventory screen
  (if isActive
    (`self.UpdateInteractionTargetCharacter` false
      (:`execOut`
        (`KismetSystemLibrary.Delay` 0.5) ; Give the widgets some time to spawn
        (bind _foundwidgets (`WidgetBlueprintLibrary.GetAllWidgetsOfClass` "/Script/ConanSandbox.PaperdollPanel" false))
        (for _array_element _foundwidgets
          (`self.MakeCASInventoryButton` (`Widget.GetParent` _array_element)))))))

(event `EventRPCUpdateSkeletalMesh`
  (params (TargetComponent :type "SkinnedMeshComponent Object Reference") (SkeletalMesh :type "SkeletalMesh Object Reference"))
  ;[1 1 1] Workaround, see https://issues.unrealengine.com/issue/UE-76862
  (`SkinnedMeshComponent.SetSkinnedAssetAndUpdate` (stale `EventUpdateSkeletalMesh` TargetComponent) SkeletalMesh true)
  (`SkinnedMeshComponent.SetSkinnedAssetAndUpdate` TargetComponent SkeletalMesh true))

(fn `CAS.GetInventoryItem`
  (params (SlotName :type String))
  (returns (EquippedItem :type "GameItem Object Reference"))
  (bind _casitem (`/Game/Mods/CAS/inventory/blueprints/BP_CAS_inventory_functions.findCASInventoryItemBySlot` (`self.CAS.Inventory`) SlotName))
  (bind _item (`/Game/Mods/CAS/inventory/blueprints/BP_CAS_inventory_functions.resolveCASItem` _casitem (`self.ParentCharacter`)))
  (return _item))

(fn `CAS.IsSlotLocked`
  (params (SlotName :type String))
  (returns (IsLocked :type Boolean))
  (locals (TargetSlotName :type String))
  (bind _output_get (set `local.TargetSlotName` SlotName))
  (if (`KismetStringLibrary.Contains` _output_get "pouch")
    (bind _item (`/Game/Mods/CAS/inventory/blueprints/BP_CAS_inventory_functions.getCurrentBelt` (`self.CAS.Inventory`) (`self.ParentCharacter`)))
    (`/Game/Systems/BP_MacroGlobal.IsValid+Branch` _item true
      (:`True`
        (bind _returnvalue (`|GetDataTableRow` "/Game/Items/ItemTable.ItemTable" (`KismetStringLibrary.Conv_StringToName` (`KismetStringLibrary.Conv_IntToString` (`GameItem.TemplateID` _item))))
          (:`then`
            (return (< (`.ItemContainerSize` (break `ItemTableRow` _returnvalue)) (`KismetStringLibrary.Conv_StringToInt` (`KismetStringLibrary.GetSubstring` (`local.TargetSlotName`) 5)))))
          (:`RowNotFound`
            (return true))))
      (:`False or Invalid`
        (return true)))
    (else
      (return false))))

(fn `CAS.RegisterItem`
  (params (Arg1 :type String) (Arg2 :type "Float (double-precision)") (Arg3 :type Integer)))

(fn `CAS.ToggleItemVisible`
  (params (Item :type "GameItem Object Reference") (Visible :type Boolean))
  (locals (CASItemBeingToggled :type "/Game/Mods/CAS/inventory/blueprints/CASInventoryItem Structure") (Visibility :type Boolean) (ItemBeingToggled :type "GameItem Object Reference"))
  (bind _parentcharacter (`self.ParentCharacter`))
  (bind _itembeingtoggled (`local.ItemBeingToggled`))
  (set `local.ItemBeingToggled` Item)
  (set `local.Visibility` Visible)
  (bind _casitem (`/Game/Mods/CAS/inventory/blueprints/BP_CAS_inventory_functions.findCASInventoryItem` (`self.CAS.Inventory`) Item))
  (set `local.CASItemBeingToggled` _casitem)
  (if (> (`KismetStringLibrary.Len` (`.GameItemID_11_07FD5B0E4AB07E5A4472A18811FFE6D4` (break `/Game/Mods/CAS/inventory/blueprints/CASInventoryItem` _casitem))) 0)
    (bind _asbp_attachable (cast `/Game/Mods/CAS/attachables/BP_attachable` _itembeingtoggled)
      (:`then`
        (`/Game/Mods/CAS/attachables/BP_attachable.ToggleAttach` _asbp_attachable _parentcharacter (`local.Visibility`)))
      (:`CastFailed`
        (bind _tag (`/Game/Mods/CAS/inventory/blueprints/BP_CAS_inventory_functions.generateItemEquipmentTag` _itembeingtoggled))
        (bind _matchedactors (`/Game/Mods/CAS/inventory/blueprints/BP_CAS_inventory_functions.findAttachedActorsByTag` _parentcharacter _tag))
        (for _array_element _matchedactors
          (`Actor.SetActorHiddenInGame` _array_element (not (`local.Visibility`))))))))

(fn `CAS.TryEquipItem`
  (params (Item :type "GameItem Object Reference") (`CAS.SlotName` :type String))
  (returns (success :type Boolean))
  (locals (ItemBeingEquipped :type "GameItem Object Reference") (ItemSlotBeingEquipped :type String) (ItemIsAlreadyInSlot :type Boolean) (AttachingActor :type "/Game/Mods/CAS/attachables/BP_attaching_actor Object Reference") (MeshComponentToPosition :type "SceneComponent Object Reference") (SocketToUse :type Name))
  (bind _parentcharacter (`self.ParentCharacter`))
  (bind _staticmesh (`/Game/Mods/CAS/attachables/BP_attaching_actor.StaticMesh` (`local.AttachingActor`)))
  (bind _skeletalmesh (`/Game/Mods/CAS/attachables/BP_attaching_actor.SkeletalMesh` (`local.AttachingActor`)))
  (bind _staticmesh_2 (`/Game/Mods/CAS/attachables/BP_attaching_actor.StaticMesh` (`local.AttachingActor`)))
  (set `local.ItemBeingEquipped` Item)
  (set `local.ItemSlotBeingEquipped` `CAS.SlotName`)
  ;[1 1 1] Pre-flight checks
  (`|ExecutionSequence`
    (:`then_0`
      (bind _valid (`/Game/Mods/CAS/inventory/blueprints/BP_CAS_inventory_functions.isValidSlot` (`local.ItemBeingEquipped`) (`local.ItemSlotBeingEquipped`) (`self.ParentCharacter`)))
      (if (not _valid)
        (return false)))
    (:`then_1`
      (bind _islocked (`self.CAS.IsSlotLocked` (`local.ItemSlotBeingEquipped`)))
      (if _islocked
        (return false)))
    (:`then_2`
      (bind _casitem (`/Game/Mods/CAS/inventory/blueprints/BP_CAS_inventory_functions.findCASInventoryItemBySlot` (`self.CAS.Inventory`) (`local.ItemSlotBeingEquipped`)))
      (bind _isvalid (`/Game/Mods/CAS/inventory/blueprints/BP_CAS_inventory_functions.isValidCASItem` _casitem))
      (if _isvalid
        (bind _uniqueid (`/Game/Mods/CAS/inventory/blueprints/BP_CAS_inventory_functions.generateItemUniqueID` (`local.ItemBeingEquipped`)))
        (if (`KismetStringLibrary.EqualEqual_StrStr` _uniqueid (`.GameItemID_11_07FD5B0E4AB07E5A4472A18811FFE6D4` (break `/Game/Mods/CAS/inventory/blueprints/CASInventoryItem` _casitem)))
          (set `local.ItemIsAlreadyInSlot` true)
          (else
            (`self.CAS.TryUnequipItem` (`local.ItemSlotBeingEquipped`))))))
    (:`then_3`
      ;[1 1 1] Hand-off for server execution
      (if (`KismetSystemLibrary.IsServer`)
        (`|ExecutionSequence`
          (:`then_0`
            ;[1 1 1] Find mesh and attach it
            (bind _tag (`/Game/Mods/CAS/inventory/blueprints/BP_CAS_inventory_functions.generateItemEquipmentTag` (`local.ItemBeingEquipped`)))
            (bind _matchedactors (`/Game/Mods/CAS/inventory/blueprints/BP_CAS_inventory_functions.findAttachedActorsByTag` (`self.ParentCharacter`) _tag))
            (if (== (`KismetArrayLibrary.Array_Length` _matchedactors) 0)
              (bind _worldcomponenttransform (`CharacterFunctionLibrary.GetWorldComponentTransform` (`Character.Mesh` (`self.ParentCharacter`))))
              (bind _asbp_attachable (cast `/Game/Mods/CAS/attachables/BP_attachable` (`local.ItemBeingEquipped`))
                (:`then`
                  (`/Game/Systems/BP_MacroGlobal.IsValid+Branch` (`/Game/Mods/CAS/attachables/BP_attachable.MeshToAttach` _asbp_attachable) true
                    (:`True`
                      (bind _returnvalue (`|SpawnActorFromClass` "/Game/Mods/CAS/attachables/BP_attaching_actor.BP_attaching_actor_C" _worldcomponenttransform "Undefined" "OverrideRootScale" :!label _label))
                      (set `local.AttachingActor` _returnvalue))
                    (:`False or Invalid`
                      (bind _returnvalue_2 (`|SpawnActorFromClass` (`/Game/Mods/CAS/attachables/BP_attachable.ActorToAttach` _asbp_attachable) _worldcomponenttransform "Undefined" "OverrideRootScale"))
                      (bind _asbp_attaching_actor (cast `/Game/Mods/CAS/attachables/BP_attaching_actor` _returnvalue_2))
                      (set `local.AttachingActor` _asbp_attaching_actor))))
                (:`CastFailed`
                  (goto _label)))
              (`KismetArrayLibrary.Array_Add` (`Actor.Tags` (`local.AttachingActor`)) (`KismetStringLibrary.Conv_StringToName` _tag))
              (bind (_transform _targetsocket) (`/Game/Mods/CAS/inventory/blueprints/BP_CAS_inventory_functions.determineItemEquipTransform` (`local.ItemBeingEquipped`) (`local.ItemSlotBeingEquipped`) (`self.ParentCharacter`)))
              (set `local.SocketToUse` _targetsocket)
              (`|ExecutionSequence`
                (:`then_0`
                  (bind _asbp_attachable_2 (cast `/Game/Mods/CAS/attachables/BP_attachable` (`local.ItemBeingEquipped`))
                    (:`then`
                      (bind _meshtoattach (`/Game/Mods/CAS/attachables/BP_attachable.MeshToAttach` _asbp_attachable_2))
                      (`/Game/Systems/BP_MacroGlobal.IsValid+Branch` _meshtoattach true
                        (:`True`
                          (`StaticMeshComponent.SetStaticMesh` _staticmesh _meshtoattach)
                          (set `local.MeshComponentToPosition` _staticmesh))
                        (:`False or Invalid`
                          (set `local.MeshComponentToPosition` (`/Game/Mods/CAS/attachables/BP_attaching_actor.SkeletalMesh` (`local.AttachingActor`)))))
                      (set `local.SocketToUse` (`/Game/Mods/CAS/attachables/BP_attachable.TargetSocket` _asbp_attachable_2)))
                    (:`CastFailed`
                      (bind (_staticmesh_3 _skeletalmesh_2) (`/Game/Mods/CAS/inventory/blueprints/BP_CAS_inventory_functions.findItemMeshToDisplay` (`local.ItemBeingEquipped`)))
                      (`/Game/Systems/BP_MacroGlobal.IsValid+Branch` _staticmesh_3 true
                        (:`True`
                          (`StaticMeshComponent.SetStaticMesh` _staticmesh_2 _staticmesh_3)
                          (set `local.MeshComponentToPosition` _staticmesh_2))
                        (:`False or Invalid`
                          (`self.EventUpdateSkeletalMesh` _skeletalmesh _skeletalmesh_2)
                          (set `local.MeshComponentToPosition` _skeletalmesh))))))
                (:`then_1`
                  (`SceneComponent.K2_SetRelativeTransform` (`local.MeshComponentToPosition`) _transform false false)
                  (`Actor.K2_AttachToComponent` (`local.AttachingActor`) (`Character.Mesh` (`self.ParentCharacter`)) (`local.SocketToUse`) "SnapToTarget" "SnapToTarget" "SnapToTarget" true)
                  (bind _asskeletal_mesh_component (cast `SkeletalMeshComponent` (`local.MeshComponentToPosition`)))
                  (`SkinnedMeshComponent.SetLeaderPoseComponent` _asskeletal_mesh_component (`Character.Mesh` (`self.ParentCharacter`)))))))
          (:`then_1`
            ;[1 1 1] Apply buffs
            (bind _asbp_cas_buff_provider (cast `/Game/Mods/CAS/buffs/BP_CAS_buff_provider` (`local.ItemBeingEquipped`)))
            (bind _buffs (`/Game/Mods/CAS/buffs/BP_CAS_buff_provider.getBuffsToApply` _asbp_cas_buff_provider))
            (for _array_element _buffs
              (`/Game/Systems/Buffs/00_BP_AC_BuffSystem.AddBuff` (`KismetArrayLibrary.Array_Get` (`Actor.K2_GetComponentsByClass` (`self.ParentCharacter`) "/Game/Systems/Buffs/00_BP_AC_BuffSystem.00_BP_AC_BuffSystem_C")) _array_element _parentcharacter 0 (`/Game/Characters/FuncomFunctionLibrary.GetControllerFromActor` _parentcharacter))))
          (:`then_2`
            ;[1 1 1] Update the CAS.Inventory
            (if (not (`local.ItemIsAlreadyInSlot`))
              (`/Game/Mods/CAS/inventory/blueprints/BP_CAS_inventory_functions.setCASInventoryItem` (`self.CAS.Inventory`) (`local.ItemSlotBeingEquipped`) (`local.ItemBeingEquipped`))))
          (:`then_3`
            (return true)))
        (else
          (bind _uniqueid_2 (`/Game/Mods/CAS/inventory/blueprints/BP_CAS_inventory_functions.generateItemUniqueID` (`local.ItemBeingEquipped`)))
          (`self.EventTryEquipItem` (`local.ItemSlotBeingEquipped`) _uniqueid_2)
          (return true))))))

(fn `CAS.TryUnequipItem`
  (params (`CAS.SlotName` :type String))
  (returns (UnequipSuccess :type Boolean))
  (locals (SlotName :type String) (ItemBeingUnequipped :type "GameItem Object Reference") (CASItemBeingUnequipped :type "/Game/Mods/CAS/inventory/blueprints/CASInventoryItem Structure"))
  (set `local.SlotName` `CAS.SlotName`)
  ;[1 1 1] Hand-off for server execution
  (if (`KismetSystemLibrary.IsServer`)
    ;[1 1 1] Remove item from CAS inventory
    (bind _previousitem (`/Game/Mods/CAS/inventory/blueprints/BP_CAS_inventory_functions.removeCASInventoryItem` (`self.CAS.Inventory`) (`local.SlotName`)))
    (bind _output_get (set `local.CASItemBeingUnequipped` _previousitem))
    (bind _item (`/Game/Mods/CAS/inventory/blueprints/BP_CAS_inventory_functions.resolveCASItem` _output_get (`self.ParentCharacter`)))
    (set `local.ItemBeingUnequipped` _item)
    (`|ExecutionSequence`
      (:`then_0`
        ;[1 1 1] Remove item visual
        (bind _tag (`/Game/Mods/CAS/inventory/blueprints/BP_CAS_inventory_functions.generateItemEquipmentTag` (`local.ItemBeingUnequipped`)))
        (bind _matchedactors (`/Game/Mods/CAS/inventory/blueprints/BP_CAS_inventory_functions.findAttachedActorsByTag` (`self.ParentCharacter`) _tag))
        (for _array_element _matchedactors
          (`Actor.K2_DestroyActor` _array_element)))
      (:`then_1`
        ;[1 1 1] Stop any buffs
        (bind _asbp_cas_buff_provider (cast `/Game/Mods/CAS/buffs/BP_CAS_buff_provider` (`local.ItemBeingUnequipped`)))
        (bind _buffs (`/Game/Mods/CAS/buffs/BP_CAS_buff_provider.getBuffsToApply` _asbp_cas_buff_provider))
        (for _array_element_2 _buffs
          (`/Game/Systems/Buffs/00_BP_AC_BuffSystem.RemoveBuff` (`KismetArrayLibrary.Array_Get` (`Actor.K2_GetComponentsByClass` (`self.ParentCharacter`) "/Game/Systems/Buffs/00_BP_AC_BuffSystem.00_BP_AC_BuffSystem_C")) _array_element_2)))
      (:`then_2`
        (return true)))
    (else
      (`self.EventTryUnequipItem` (`local.SlotName`))
      (return true))))