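; Function library for the CAS inventory, which places character items in named slots and resolves how they display.
; Slot entries store template IDs as provisional unique IDs, resolved against backpack, shortcut bar and equipment inventories.
; Data tables supply weapon and gendered armor meshes, plus slot sockets and transforms, adjusted by wildcard-matched overrides.
; Helpers validate slots, find attached actors by tag and read gender from the anim instance.
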(fn `createCASItem`
  (params (SlotName :type String) (ItemID :type String))
  (returns (CASItem :type "/Game/Mods/CAS/inventory/blueprints/CASInventoryItem Structure"))
  (return (make `/Game/Mods/CAS/inventory/blueprints/CASInventoryItem` SlotName ItemID)))

(fn `determineItemEquipTransform`
  (params (item :type "GameItem Object Reference") (slotName :type String) (character :type "/Game/Characters/BaseBPChar Object Reference"))
  (returns (transform :type "Transform Structure") (targetSocket :type Name))
  (locals (TransformToApply :type "Transform Structure") (SocketToUse :type String :default "b_root") (CASSlotName :type String) (ItemToEquip :type "GameItem Object Reference") (TargetCharacter :type "/Game/Characters/BaseBPChar Object Reference") (TargetIsFemale :type Boolean) (ItemVisualObjectClassName :type String))
  (set `local.ItemToEquip` item)
  (set `local.CASSlotName` slotName)
  (bind _output_get (set `local.TargetCharacter` character))
  (bind _isfemale (`self.getCharacterGender` _output_get))
  (set `local.TargetIsFemale` _isfemale)
  (`|ExecutionSequence`
    (:`then_0`
      ;[1 1 1] Look up the initial transform from the slot table
      (bind _returnvalue (`|GetDataTableRow` "/Game/Mods/CAS/inventory/CAS_SlotTable.CAS_SlotTable" (`KismetStringLibrary.Conv_StringToName` (`local.CASSlotName`)))
        (:`then`
          (bind (_transformmale _transformfemale _targetsocket) (break `/Game/Mods/CAS/inventory/CAS_SlotTableRow` _returnvalue))
          (set `local.TransformToApply` (`KismetMathLibrary.SelectTransform` _transformfemale _transformmale (`local.TargetIsFemale`)))
          (set `local.SocketToUse` _targetsocket))))
    (:`then_1`
      ;[1 1 1] Figure out the item's VisualObjectClassName, if any
      (bind _returnvalue_2 (`|GetDataTableRow` "/Game/Items/ItemTable.ItemTable" (`KismetStringLibrary.Conv_StringToName` (`KismetStringLibrary.Conv_IntToString` (`GameItem.TemplateID` (`local.ItemToEquip`)))))
        (:`then`
          (bind _asbase_weapon (castclass `/Game/Items/Weapons/BaseWeapon` (`|ConvertAsset` (`.VisualObject` (break `ItemTableRow` _returnvalue_2)))))
          (set `local.ItemVisualObjectClassName` (`KismetSystemLibrary.GetClassDisplayName` _asbase_weapon)))))
    (:`then_2`
      ;[1 1 1] Apply any transform overrides from the override table
      (bind _outrownames (`DataTableFunctionLibrary.GetDataTableRowNames` "/Game/Mods/CAS/inventory/CAS_ItemOverrideTable.CAS_ItemOverrideTable"))
      (for _array_element _outrownames
        (bind _returnvalue_3 (`|GetDataTableRow` "/Game/Mods/CAS/inventory/CAS_ItemOverrideTable.CAS_ItemOverrideTable" _array_element)
          (:`then`
            (bind (_visualobjectnamepattern _casslotnamepattern _genderpattern _transform _targetsocket_2) (break `/Game/Mods/CAS/inventory/CAS_ItemOverrideTableRow` _returnvalue_3))
            (if (and (`KismetStringLibrary.MatchesWildcard` (`local.ItemVisualObjectClassName`) _visualobjectnamepattern) (`KismetStringLibrary.MatchesWildcard` (`local.CASSlotName`) _casslotnamepattern) (`KismetStringLibrary.MatchesWildcard` (`KismetMathLibrary.SelectString` "female" "male" (`local.TargetIsFemale`)) _genderpattern))
              (set `local.TransformToApply` (`KismetMathLibrary.ComposeTransforms` _transform (`local.TransformToApply`)))
              (if (> (`KismetStringLibrary.Len` _targetsocket_2) 0)
                (set `local.SocketToUse` _targetsocket_2)))))))
    (:`then_3`
      (return (`local.TransformToApply`) (`KismetStringLibrary.Conv_StringToName` (`local.SocketToUse`))))))

(fn `findAttachedActorsByTag`
  (params (character :type "/Game/Characters/BaseBPChar Object Reference") (tag :type String))
  (returns (matchedActors :type "Array of Actor Object Reference"))
  (locals (MatchingActors :type "Array of Actor Object Reference"))
  (for _array_element (`Actor.GetAttachedActors` character)
    (for _array_element_2 (`Actor.Tags` _array_element)
      (if (`KismetStringLibrary.EqualEqual_StrStr` (`KismetStringLibrary.Conv_NameToString` _array_element_2) tag)
        (`KismetArrayLibrary.Array_Add` (`local.MatchingActors`) _array_element)
        (break))))
  (return (`local.MatchingActors`)))

(fn `findCASInventoryItem`
  (params (Inventory :type "Array of /Game/Mods/CAS/inventory/blueprints/CASInventoryItem Structure") (Item :type "GameItem Object Reference"))
  (returns (CASItem :type "/Game/Mods/CAS/inventory/blueprints/CASInventoryItem Structure"))
  (locals (MatchingItem :type "/Game/Mods/CAS/inventory/blueprints/CASInventoryItem Structure"))
  (bind _uniqueid (`self.generateItemUniqueID` Item))
  (for _array_element Inventory
    (if (`KismetStringLibrary.EqualEqual_StrStr` _uniqueid (`.GameItemID_11_07FD5B0E4AB07E5A4472A18811FFE6D4` (break `/Game/Mods/CAS/inventory/blueprints/CASInventoryItem` _array_element)))
      (set `local.MatchingItem` _array_element)
      (break)))
  (return (`local.MatchingItem`)))

(fn `findCASInventoryItemBySlot`
  (params (Inventory :type "Array of /Game/Mods/CAS/inventory/blueprints/CASInventoryItem Structure") (SlotName :type String))
  (returns (CASItem :type "/Game/Mods/CAS/inventory/blueprints/CASInventoryItem Structure"))
  (locals (MatchingItem :type "/Game/Mods/CAS/inventory/blueprints/CASInventoryItem Structure"))
  (for _array_element Inventory
    (if (`KismetStringLibrary.EqualEqual_StrStr` (`.SlotName_2_8DC5705C4B2832C95D9D0A8F1CA76B34` (break `/Game/Mods/CAS/inventory/blueprints/CASInventoryItem` _array_element)) SlotName)
      (set `local.MatchingItem` _array_element)
      (break)))
  (return (`local.MatchingItem`)))

(fn `findCharacterInventoryItem`
  (params (Character :type "/Game/Characters/BaseBPChar Object Reference") (ItemID :type Integer))
  (returns (Item :type "GameItem Object Reference"))
  (locals (TemplateID :type Integer) (CharacterBeingSearched :type "/Game/Characters/BaseBPChar Object Reference"))
  (bind _characterbeingsearched (`local.CharacterBeingSearched`))
  (set `local.CharacterBeingSearched` Character)
  (bind _output_get (set `local.TemplateID` ItemID))
  (if (> _output_get 0)
    (`|ExecutionSequence`
      (:`then_0`
        (bind _returnvalue (`ConanCharacter.GetBackpackInventory` _characterbeingsearched))
        (bind _returnvalue_2 (`ItemInventory.GetItem` _returnvalue (`ItemInventory.FindItemByTemplateID` _returnvalue (`local.TemplateID`) 0)))
        (`/Game/Systems/BP_MacroGlobal.IsValid+Branch` _returnvalue_2 true
          (:`True`
            (return _returnvalue_2))))
      (:`then_1`
        (bind _returnvalue_3 (`ConanCharacter.GetShortcutBarInventory` _characterbeingsearched))
        (bind _returnvalue_4 (`ItemInventory.GetItem` _returnvalue_3 (`ItemInventory.FindItemByTemplateID` _returnvalue_3 (`local.TemplateID`) 0)))
        (`/Game/Systems/BP_MacroGlobal.IsValid+Branch` _returnvalue_4 true
          (:`True`
            (return _returnvalue_4))))
      (:`then_2`
        (bind _returnvalue_5 (`ConanCharacter.GetEquipmentInventoryNative` _characterbeingsearched))
        (bind _returnvalue_6 (`ItemInventory.GetItem` _returnvalue_5 (`ItemInventory.FindItemByTemplateID` _returnvalue_5 (`local.TemplateID`) 0)))
        (`/Game/Systems/BP_MacroGlobal.IsValid+Branch` _returnvalue_6 true
          (:`True`
            (return _returnvalue_6))))
      (:`then_3`
        _)))
  (return null))

(fn `findItemMeshToDisplay`
  (params (GameItem :type "GameItem Object Reference") (TargetCharacter :type "/Game/Characters/BaseBPChar Object Reference"))
  (returns (StaticMesh :type "StaticMesh Object Reference") (SkeletalMesh :type "SkeletalMesh Object Reference"))
  (locals (GameItemToCheck :type "GameItem Object Reference") (TargetCharacterToCheck :type "/Game/Characters/BaseBPChar Object Reference"))
  (set `local.GameItemToCheck` GameItem)
  (set `local.TargetCharacterToCheck` TargetCharacter)
  (`|ExecutionSequence`
    (:`then_0`
      (bind _asbpgame_item_weapon (cast `/Game/Items/BPGameItemWeapon` (`local.GameItemToCheck`)))
      (bind _returnvalue (`|GetDataTableRow` "/Game/Items/ItemTable.ItemTable" (`KismetStringLibrary.Conv_StringToName` (`KismetStringLibrary.Conv_IntToString` (`GameItem.TemplateID` _asbpgame_item_weapon))))
        (:`then`
          (bind (_name _shortdesc _longdesc _icon _itemclass _buildingclass _visualobject _actionblueprint_use _maxstacksize _equiplocation _guicategory _armourvalue _armortype _soundphysicalsurface _weapontype _weaponarchetype _compatableammunitions _soundtransmittertype _knockbackresponseweapon _weaponstaminaattacksinglebasic _weaponstaminaattacksinglespecial _weaponstaminaattackdualbasic _weaponstaminaattackdualspecial _weaponstaminaheavychargedregenmodifier _weaponspeedheavychargedmodifier _encumbranceweight _coneangle _conemaxdistance _damagehealthlight_onhit _damagehealthheavy_onhit _damagestaminalight_onhit _damagestaminaheavy_onhit _damagehealthlight_onblock _damagehealthheavy_onblock _damagestaminalight_onblock _damagestaminaheavy_onblock _harvestdamage _weaponusage _maxattackreach _minattackreach _minattackdistance _weaponeffectwidth _weaponeffectheight _itemtier _armorpen _damageconcussivelightonhit _damageconcussiveheavyonhit _damageconcussivelightonblock _damageconcussiveheavyonblock _damagetier _cooldowntime _reusetime _selectionweight _knockbackoffensebasic _knockbackoffensespecial _knockbackoffensebasiconblock _knockbackoffensespecialonblock _knockbackdefense _visualstaticmesh _visualskeletalmesh) (break `ItemTableRow` _returnvalue))
          (`/Engine/EditorBlueprintResources/StandardMacros.IsAssetValid` _visualstaticmesh
            (:`IsValid`
              (bind _returnvalue_2 (`FuncomGenericLibrary.SyncLoadAsset` _visualstaticmesh))
              (bind _asstatic_mesh (cast `StaticMesh` _returnvalue_2))
              (return _asstatic_mesh null))
            (:`Is Not Valid`
              (`/Engine/EditorBlueprintResources/StandardMacros.IsAssetValid` _visualskeletalmesh
                (:`IsValid`
                  (bind _returnvalue_3 (`FuncomGenericLibrary.SyncLoadAsset` _visualskeletalmesh))
                  (bind _asskeletal_mesh (cast `SkeletalMesh` _returnvalue_3))
                  (return null _asskeletal_mesh))))))))
    (:`then_1`
      (bind _asbpgame_item_armor (cast `/Game/Items/BPGameItemArmor` (`local.GameItemToCheck`)))
      (bind _returnvalue_4 (`|GetDataTableRow` "/Game/Items/EquipmentVariationTable.EquipmentVariationTable" (`KismetStringLibrary.Conv_StringToName` (`KismetStringLibrary.Conv_IntToString` (`GameItem.TemplateID` _asbpgame_item_armor))))
        (:`then`
          (bind _isfemale (`self.getCharacterGender` (`local.TargetCharacterToCheck`)))
          (bind (_slottype _malepath _femalepath) (break `EquipmentGenderVariations` _returnvalue_4))
          (bind _returnvalue_5 (select `bool` _isfemale :`false` _malepath :`true` _femalepath))
          (`/Engine/EditorBlueprintResources/StandardMacros.IsAssetValid` _returnvalue_5
            (:`IsValid`
              (bind _returnvalue_6 (`FuncomGenericLibrary.SyncLoadAsset` _returnvalue_5))
              (bind _asskeletal_mesh_2 (cast `SkeletalMesh` _returnvalue_6))
              (return null _asskeletal_mesh_2))))))
    (:`then_2`
      (return null null))))

(fn `generateItemEquipmentTag`
  (params (Item :type "GameItem Object Reference"))
  (returns (tag :type String))
  (bind _uniqueid (`self.generateItemUniqueID` Item))
  (return (`KismetStringLibrary.Concat_StrStr` "CAS.Attached." _uniqueid)))

(fn `generateItemUniqueID`
  (params (Item :type "GameItem Object Reference"))
  (returns (UniqueID :type String))
  (return (`KismetStringLibrary.Conv_IntToString` (`GameItem.TemplateID` Item))))

(fn `getCharacterGender`
  (params (Character :type "/Game/Characters/BaseBPChar Object Reference"))
  (returns (IsFemale :type Boolean))
  (bind _asab_human_male (cast `/Game/Master_AnimBP/AB_human_male` (`SkeletalMeshComponent.GetAnimInstance` (`Character.Mesh` Character)))
    (:`then`
      (return (`/Game/Master_AnimBP/AB_human_male.IsFemale` _asab_human_male)))
    (:`CastFailed`
      (return false))))

(fn `getCurrentBelt`
  (params (Inventory :type "Array of /Game/Mods/CAS/inventory/blueprints/CASInventoryItem Structure") (character :type "/Game/Characters/BaseBPChar Object Reference"))
  (returns (Item :type "GameItem Object Reference") (CASItem :type "/Game/Mods/CAS/inventory/blueprints/CASInventoryItem Structure"))
  (locals (MatchingItem :type "/Game/Mods/CAS/inventory/blueprints/CASInventoryItem Structure"))
  (bind _casitem (`self.findCASInventoryItemBySlot` Inventory "belt"))
  (bind _item (`self.resolveCASItem` _casitem character))
  (return _item _casitem))

(fn `hasEquipmentTag`
  (params (tags :type "Array of Name") (CASItem :type "/Game/Mods/CAS/inventory/blueprints/CASInventoryItem Structure") (character :type "/Game/Characters/BaseBPChar Object Reference"))
  (returns (hasTag :type Boolean))
  (bind _item (`self.resolveCASItem` CASItem character))
  (bind _tag (`self.generateItemEquipmentTag` _item))
  (for _array_element tags
    (if (`KismetStringLibrary.EqualEqual_StrStr` _tag (`KismetStringLibrary.Conv_NameToString` _array_element))
      (return true)))
  (return false))

(fn `isValidCASItem`
  (params (CASItem :type "/Game/Mods/CAS/inventory/blueprints/CASInventoryItem Structure"))
  (returns (isValid :type Boolean))
  (return (> (`KismetStringLibrary.Len` (`.GameItemID_11_07FD5B0E4AB07E5A4472A18811FFE6D4` (break `/Game/Mods/CAS/inventory/blueprints/CASInventoryItem` CASItem))) 0)))

(fn `isValidSlot`
  (params (item :type "GameItem Object Reference") (slotName :type String) (character :type "/Game/Characters/BaseBPChar Object Reference"))
  (returns (valid :type Boolean))
  (`|ExecutionSequence`
    (:`then_0`
      ;[1 1 1] Weapons: May only go into weapon slots
      (cast `/Game/Items/BPGameItemWeapon` item)
      (return (`KismetStringLibrary.Contains` slotName "weapon")))
    (:`then_1`
      ;[1 1 1] Attachables: May go anywhere
      (cast `/Game/Mods/CAS/attachables/BP_attachable` item)
      (return true))
    (:`then_2`
      ;[1 1 1] Misc Slots: Accept any item
      (return (`KismetStringLibrary.Contains` slotName "misc")))))

(fn `removeCASInventoryItem`
  (params (Inventory :type "Array of /Game/Mods/CAS/inventory/blueprints/CASInventoryItem Structure") (SlotName :type String))
  (returns (PreviousItem :type "/Game/Mods/CAS/inventory/blueprints/CASInventoryItem Structure"))
  (locals (MatchingItem :type "/Game/Mods/CAS/inventory/blueprints/CASInventoryItem Structure") (MatchingItemIndex :type Integer :default -1))
  (for (_array_element _array_index) Inventory
    (if (`KismetStringLibrary.EqualEqual_StrStr` (`.SlotName_2_8DC5705C4B2832C95D9D0A8F1CA76B34` (break `/Game/Mods/CAS/inventory/blueprints/CASInventoryItem` _array_element)) SlotName)
      (set `local.MatchingItem` _array_element)
      (set `local.MatchingItemIndex` _array_index)
      (break)))
  (if (>= (`local.MatchingItemIndex`) 0)
    (`KismetArrayLibrary.Array_Remove` Inventory (`local.MatchingItemIndex`)))
  (return (`local.MatchingItem`)))

(fn `resolveCASItem`
  (params (CASItem :type "/Game/Mods/CAS/inventory/blueprints/CASInventoryItem Structure") (Character :type "/Game/Characters/BaseBPChar Object Reference"))
  (returns (Item :type "GameItem Object Reference"))
  (bind _item (`self.findCharacterInventoryItem` Character (`KismetStringLibrary.Conv_StringToInt` (`.GameItemID_11_07FD5B0E4AB07E5A4472A18811FFE6D4` (break `/Game/Mods/CAS/inventory/blueprints/CASInventoryItem` CASItem)))))
  (return _item))

(fn `setCASInventoryItem`
  (params (Inventory :type "Array of /Game/Mods/CAS/inventory/blueprints/CASInventoryItem Structure") (SlotName :type String) (ItemToEquip :type "GameItem Object Reference"))
  (returns (PreviousItem :type "GameItem Object Reference"))
  (locals (ExistingItemInSlot :type "GameItem Object Reference"))
  (`self.removeCASInventoryItem` Inventory SlotName)
  (bind _uniqueid (`self.generateItemUniqueID` ItemToEquip))
  (bind _casitem (`self.createCASItem` SlotName _uniqueid))
  (`KismetArrayLibrary.Array_Add` Inventory _casitem)
  (return null))