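; Character component for CAS, an equipment system that attaches item visuals to players and thralls in named slots.
; The server validates slots (pouches depend on belt or backpack), spawns tagged attaching actors, applies buffs, updates the persistent CAS inventory and re-equips it after BeginPlay.
; Inventory signals hide visuals of equipped items and unequip items leaving the character.
; Clients get CAS buttons in inventory screens; thrall equip calls route through RPC wrappers.
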(event `EventItemAdded`
  (params (index :type Integer) (item :type "GameItem Object Reference") (srcInventory :type "ItemInventory Object Reference") (srcIndex :type Integer))
  ;[1 1 1] Listen for weapon sheathing events
  (`self.CAS.ToggleItemVisible` item))

(event `EventItemRemoved`
  (params (index :type Integer) (item :type "GameItem Object Reference") (dstInventory :type "ItemInventory Object Reference") (dstIndex :type Integer))
  ;[1 1 1] Listen for weapon sheathing events
  (`self.CAS.ToggleItemVisible` item true))

(event `EventItemRemovedCheckDrop`
  (params (index :type Integer) (item :type "GameItem Object Reference") (dstInventory :type "ItemInventory Object Reference") (dstIndex :type Integer))
  ;[1 1 1] Listen for item dropping events
  (`self.CAS.CheckItemDropped` item dstInventory))

(event `self.ReceiveBeginPlay`
  (bind _returnvalue (`KismetArrayLibrary.Array_Length` (`self.CAS.Inventory`)))
  (bind _inventory (`/Game/Characters/BaseBPChar.GetEquipmentInventory` (`self.ParentCharacter`)))
  (bind _asbase_bpchar (cast `/Game/Characters/BaseBPChar` (`self.GetOwner`)))
  (set `self.ParentCharacter` _asbase_bpchar)
  (`KismetSystemLibrary.Delay` 3.0) ; Give some time before we can assume replication is in place
  (`|ExecutionSequence`
    (:`then_0`
      (if (`KismetSystemLibrary.IsServer`)
        (`|ExecutionSequence`
          (:`then_0`
            ;[1 1 1] Listen for weapon sheathing events
            (add `ItemInventory.SignalItemAdded` _inventory (delegate `EventItemAdded`))
            (add `ItemInventory.SignalItemRemoved` _inventory (delegate `EventItemRemoved`)))
          (:`then_1`
            ;[1 1 1] Listen for item dropping events
            (`|ExecutionSequence`
              (:`then_0`
                (bind _returnvalue_2 (`ConanCharacter.GetBackpackInventory` (`self.ParentCharacter`)))
                (add `ItemInventory.SignalItemRemoved` _returnvalue_2 (delegate `EventItemRemovedCheckDrop`)))
              (:`then_1`
                (bind _returnvalue_3 (`ConanCharacter.GetShortcutBarInventory` (`self.ParentCharacter`)))
                (`/Game/Systems/BP_MacroGlobal.IsValid+Branch` _returnvalue_3 true
                  (:`True`
                    (add `ItemInventory.SignalItemRemoved` _returnvalue_3 (delegate `EventItemRemovedCheckDrop`)))))
              (:`then_2`
                (bind _returnvalue_4 (`ConanCharacter.GetEquipmentInventoryNative` (`self.ParentCharacter`)))
                (add `ItemInventory.SignalItemRemoved` _returnvalue_4 (delegate `EventItemRemovedCheckDrop`)))))
          (:`then_2`
            ;[1 1 1] Re-equip all saved CAS items
            (if (> _returnvalue 0)
              (for _index (range _returnvalue)
                (bind _item (`KismetArrayLibrary.Array_Get` (`self.CAS.Inventory`) _index))
                (bind _item_2 (`/Game/Mods/CAS/inventory/BP_CAS_inventory_functions.CAS.item.resolveOnChar` _item (`self.ParentCharacter`)))
                (`self.CAS.TryEquipItem` _item_2 (`.SlotName_2_8DC5705C4B2832C95D9D0A8F1CA76B34` (break `/Game/Mods/CAS/inventory/CASInventoryItem` _item)))))))))
    (:`then_1`
      (`/Game/Systems/BP_MacroGlobal.IsValid+Branch` (`/Game/Characters/FuncomFunctionLibrary.GetControllerFromActor` (`self.ParentCharacter`)) (not (`KismetSystemLibrary.IsDedicatedServer`))
        (:`True`
          (`|ExecutionSequence`
            (:`then_0`
              ;[1 1 1] Hook a CAS button into the player's Inventory screen
              (bind _returnvalue_5 (`GUIModuleController.GetModule` (`GUIModuleController.GetGUIModuleController`) "CharacterInventory"))
              (add `GUIModule.SignalActivated` _returnvalue_5 (delegate `OnInventoryActivated`)))
            (:`then_1`
              ;[1 1 1] Hook a CAS button into the thrall Inventory screen
              (bind _returnvalue_6 (`GUIModuleController.GetModule` (`GUIModuleController.GetGUIModuleController`) "CraftingGUI"))
              (add `GUIModule.SignalActivated` _returnvalue_6 (delegate `OnThrallInvActivated`)))))))))

(event `OnInventoryActivated`
  (params (module :type "GUIModule Object Reference") (isActive :type Boolean))
  ;[1 1 1] Hook a CAS button into the player's Inventory screen
  (if isActive
    (`self.UpdateInteractionTargetCharacter` true
      (:`execOut`
        (`KismetSystemLibrary.Delay` 0.5) ; Give the widgets some time to spawn
        (`|ExecutionSequence`
          (:`then_0`
            (bind _foundwidgets (`WidgetBlueprintLibrary.GetAllWidgetsOfClass` "/Script/ConanSandbox.UICharacterDisplay" false))
            (for _array_element _foundwidgets
              (`self.MakeCASInventoryButton` (`Widget.GetParent` (`Widget.GetParent` _array_element))))))))))

(event `OnThrallInvActivated`
  (params (module :type "GUIModule Object Reference") (isActive :type Boolean))
  ;[1 1 1] Hook a CAS button into the thrall Inventory screen
  (if isActive
    (`self.UpdateInteractionTargetCharacter` false
      (:`execOut`
        (`KismetSystemLibrary.Delay` 0.5) ; Give the widgets some time to spawn
        (bind _foundwidgets (`WidgetBlueprintLibrary.GetAllWidgetsOfClass` "/Script/ConanSandbox.PaperdollPanel" false))
        (for _array_element _foundwidgets
          (`self.MakeCASInventoryButton` (`Widget.GetParent` _array_element)))))))

(event `self.ReceiveEndPlay`
  (params (EndPlayReason :type "EEndPlayReason Enum" :default "Destroyed"))
  (if (`KismetSystemLibrary.IsServer`)
    (`self.PrintDebug` "Ending play for " (`KismetSystemLibrary.GetDisplayName` (`self.ParentCharacter`)) "Cleaning up attached actors"
      (:`execOut`
        (bind _matchedactors (`/Game/Mods/CAS/inventory/BP_CAS_inventory_functions.CAS.char.findAttachedActorsByTag` (`self.ParentCharacter`) "CAS.attached.*"))
        (bind (_arrayindex _arrayelement) (`/Engine/EditorBlueprintResources/StandardMacros.ReverseForEachLoop` _matchedactors)
          (:`LoopBody`
            (`Actor.K2_DestroyActor` _arrayelement)))))))

(event `DispatchEventItemEquipped`
  (params (item :type "GameItem Object Reference") (slot :type String))
  ;[1 1 1] CAS Equipment events: multicast to all
  (`self.EventItemEquipped` item slot))

(event `DispatchEventItemUnequipped`
  (params (item :type "GameItem Object Reference") (slot :type String))
  ;[1 1 1] CAS Equipment events: multicast to all
  (`self.EventItemUnequipped` item slot))

(event `EventTryEquipItem`
  (params (SlotName :type String) (ItemID :type String))
  ;[1 1 1] RPC wrappers for equip/unequip functions to have them run on server
  (bind _casitem (`/Game/Mods/CAS/inventory/BP_CAS_inventory_functions.CAS.item.createNew` SlotName ItemID))
  (bind _item (`/Game/Mods/CAS/inventory/BP_CAS_inventory_functions.CAS.item.resolveOnChar` _casitem (`self.ParentCharacter`)))
  (`self.CAS.TryEquipItem` _item SlotName))

(event `EventTryUnequipItem`
  (params (SlotName :type String))
  ;[1 1 1] RPC wrappers for equip/unequip functions to have them run on server
  (`self.CAS.TryUnequipItem` SlotName))

(event `EventTryEquipItemOnThrall`
  (params (SlotName :type String) (ItemID :type String) (TargetCharacter :type "/Game/Characters/BaseBPChar Object Reference"))
  ;[1 1 1] RPC wrappers for equip/unequip functions to have them run on server
  (bind _casitem (`/Game/Mods/CAS/inventory/BP_CAS_inventory_functions.CAS.item.createNew` SlotName ItemID))
  (bind _item (`/Game/Mods/CAS/inventory/BP_CAS_inventory_functions.CAS.item.resolveOnChar` _casitem TargetCharacter))
  (`self.CAS.TryEquipItemOnThrall` _item SlotName TargetCharacter))

(event `EventTryUnequipItemOnThrall`
  (params (SlotName :type String) (TargetCharacter :type "/Game/Characters/BaseBPChar Object Reference"))
  ;[1 1 1] RPC wrappers for equip/unequip functions to have them run on server
  (`self.CAS.TryUnequipItemOnThrall` SlotName TargetCharacter))

(fn `CAS.CheckItemDropped`
  (params (item :type "GameItem Object Reference") (dstInventory :type "ItemInventory Object Reference"))
  (if (and (not (== (`GameplayStatics.GetObjectClass` item) "/Script/ConanSandbox.ShortcutRefItem")) (`KismetSystemLibrary.IsServer`))
    (bind _returnvalue (`ItemInventory.GetConanCharacterOwner` dstInventory))
    (`/Game/Systems/BP_MacroGlobal.IsValid+Branch` _returnvalue true
      (:`True`
        (if (not (== _returnvalue (`self.ParentCharacter`)))
          (bind _casitem (`/Game/Mods/CAS/inventory/BP_CAS_inventory_functions.CAS.inventory.findItem` (`self.CAS.Inventory`) item :!label _label))
          (bind _isvalid (`/Game/Mods/CAS/inventory/BP_CAS_inventory_functions.CAS.item.isValid` _casitem))
          (if _isvalid
            (`self.CAS.TryUnequipItem` (`.SlotName_2_8DC5705C4B2832C95D9D0A8F1CA76B34` (break `/Game/Mods/CAS/inventory/CASInventoryItem` _casitem))))))
      (:`False or Invalid`
        (goto _label)))))

(fn `CAS.GetInventoryItem`
  (params (SlotName :type String))
  (returns (EquippedItem :type "GameItem Object Reference"))
  (bind _casitem (`/Game/Mods/CAS/inventory/BP_CAS_inventory_functions.CAS.inventory.getItemInSlot` (`self.CAS.Inventory`) SlotName))
  (bind _item (`/Game/Mods/CAS/inventory/BP_CAS_inventory_functions.CAS.item.resolveOnChar` _casitem (`self.ParentCharacter`)))
  (return _item))

(fn `CAS.IsSlotLocked`
  (params (SlotName :type String))
  (returns (IsLocked :type Boolean))
  (locals (TargetSlotName :type String))
  (set `local.TargetSlotName` SlotName)
  (`|ExecutionSequence`
    (:`then_0`
      (if (`KismetStringLibrary.Contains` (`local.TargetSlotName`) "pouch")
        (bind _item (`/Game/Mods/CAS/inventory/BP_CAS_inventory_functions.CAS.inventory.getCurrentBelt` (`self.CAS.Inventory`) (`self.ParentCharacter`)))
        (`/Game/Systems/BP_MacroGlobal.IsValid+Branch` _item true
          (:`True`
            (bind _rowname (`/Game/Mods/CAS/inventory/BP_CAS_inventory_functions.CAS.gameItem.getRowName` _item))
            (bind _returnvalue (`|GetDataTableRow` "/Game/Items/ItemTable.ItemTable" _rowname)
              (:`then`
                (return (< (`.ItemContainerSize` (break `ItemTableRow` _returnvalue)) (`KismetStringLibrary.Conv_StringToInt` (`KismetStringLibrary.GetSubstring` (`local.TargetSlotName`) 5)))))
              (:`RowNotFound`
                (return true))))
          (:`False or Invalid`
            (return true)))))
    (:`then_1`
      (if (`KismetStringLibrary.Contains` (`local.TargetSlotName`) "backpackslot")
        (bind _item_2 (`/Game/Mods/CAS/inventory/BP_CAS_inventory_functions.CAS.inventory.getCurrentBackpack` (`self.CAS.Inventory`) (`self.ParentCharacter`)))
        (`/Game/Systems/BP_MacroGlobal.IsValid+Branch` _item_2 true
          (:`True`
            (bind _rowname_2 (`/Game/Mods/CAS/inventory/BP_CAS_inventory_functions.CAS.gameItem.getRowName` _item_2))
            (bind _returnvalue_2 (`|GetDataTableRow` "/Game/Items/ItemTable.ItemTable" _rowname_2)
              (:`then`
                (return (< (`.ItemContainerSize` (break `ItemTableRow` _returnvalue_2)) (`KismetStringLibrary.Conv_StringToInt` (`KismetStringLibrary.GetSubstring` (`local.TargetSlotName`) 12)))))
              (:`RowNotFound`
                (return true))))
          (:`False or Invalid`
            (return true)))))
    (:`then_2`
      (return false))))

(fn `CAS.ToggleItemVisible`
  (params (Item :type "GameItem Object Reference") (Visible :type Boolean))
  (locals (CASItemBeingToggled :type "/Game/Mods/CAS/inventory/CASInventoryItem Structure") (Visibility :type Boolean) (ItemBeingToggled :type "GameItem Object Reference"))
  (bind _output_get (set `local.ItemBeingToggled` Item))
  (set `local.Visibility` Visible)
  (bind _casitem (`/Game/Mods/CAS/inventory/BP_CAS_inventory_functions.CAS.inventory.findItem` (`self.CAS.Inventory`) _output_get))
  (set `local.CASItemBeingToggled` _casitem)
  (if (> (`KismetStringLibrary.Len` (`.GameItemID_11_07FD5B0E4AB07E5A4472A18811FFE6D4` (break `/Game/Mods/CAS/inventory/CASInventoryItem` _casitem))) 0)
    (bind _tag (`/Game/Mods/CAS/inventory/BP_CAS_inventory_functions.CAS.gameItem.generateTag` (`local.ItemBeingToggled`)))
    (bind _matchedactors (`/Game/Mods/CAS/inventory/BP_CAS_inventory_functions.CAS.char.findAttachedActorsByTag` (`self.ParentCharacter`) _tag))
    (for _array_element _matchedactors
      (`Actor.SetActorHiddenInGame` _array_element (not (`local.Visibility`))))))

(fn `CAS.TryEquipItem`
  (params (Item :type "GameItem Object Reference") (`CAS.SlotName` :type String))
  (returns (success :type Boolean))
  (locals (ItemBeingEquipped :type "GameItem Object Reference") (ItemSlotBeingEquipped :type String) (ItemIsAlreadyInSlot :type Boolean) (AttachingActor :type "/Game/Mods/CAS/attachables/BP_attaching_actor Object Reference") (MeshComponentToPosition :type "SceneComponent Object Reference") (SocketToUse :type Name) (TransformToUse :type "Transform Structure") (AttachingActorClass :type "Actor Class Reference" :default "BlueprintGeneratedClass'/Game/Mods/CAS/attachables/BP_attaching_actor.BP_attaching_actor_C'"))
  (bind _attachingactor (`local.AttachingActor`))
  (bind _attachingactor_2 (`local.AttachingActor`))
  (bind _itemslotbeingequipped (`local.ItemSlotBeingEquipped`))
  (bind _parentcharacter (`self.ParentCharacter`))
  (set `local.ItemBeingEquipped` Item)
  (set `local.ItemSlotBeingEquipped` `CAS.SlotName`)
  (if (`KismetSystemLibrary.IsServer`)
    (`self.PrintDebug` "TryEquipItem" (`KismetSystemLibrary.GetDisplayName` (`self.ParentCharacter`)) (`KismetSystemLibrary.GetDisplayName` (`local.ItemBeingEquipped`)) (`local.ItemSlotBeingEquipped`)
      (:`execOut`
        ;[1 1 1] Pre-flight checks
        (`|ExecutionSequence`
          (:`then_0`
            (bind _valid (`/Game/Mods/CAS/inventory/BP_CAS_inventory_functions.CAS.inventory.isValidSlot` (`local.ItemBeingEquipped`) _itemslotbeingequipped))
            (if (not _valid)
              (return false)))
          (:`then_1`
            (bind _islocked (`self.CAS.IsSlotLocked` _itemslotbeingequipped))
            (if _islocked
              (return false)))
          (:`then_2`
            (`|ExecutionSequence`
              (:`then_1`
                ;[1 1 1] Unequip current item, if any
                (bind _casitem (`/Game/Mods/CAS/inventory/BP_CAS_inventory_functions.CAS.inventory.getItemInSlot` (`self.CAS.Inventory`) (`local.ItemSlotBeingEquipped`)))
                (bind _isvalid (`/Game/Mods/CAS/inventory/BP_CAS_inventory_functions.CAS.item.isValid` _casitem))
                (if _isvalid
                  (bind _uniqueid (`/Game/Mods/CAS/inventory/BP_CAS_inventory_functions.CAS.gameitem.generateUID` (`local.ItemBeingEquipped`)))
                  (if (`KismetStringLibrary.EqualEqual_StrStr` _uniqueid (`.GameItemID_11_07FD5B0E4AB07E5A4472A18811FFE6D4` (break `/Game/Mods/CAS/inventory/CASInventoryItem` _casitem)))
                    (set `local.ItemIsAlreadyInSlot` true)
                    (else
                      (`self.CAS.TryUnequipItem` (`local.ItemSlotBeingEquipped`))))))
              (:`then_2`
                ;[1 1 1] Create Attaching Actor (visuals), but only if one doesn't exist already
                (bind _tag (`/Game/Mods/CAS/inventory/BP_CAS_inventory_functions.CAS.gameItem.generateTag` (`local.ItemBeingEquipped`)))
                (bind _matchedactors (`/Game/Mods/CAS/inventory/BP_CAS_inventory_functions.CAS.char.findAttachedActorsByTag` (`self.ParentCharacter`) _tag))
                (if (== (`KismetArrayLibrary.Array_Length` _matchedactors) 0)
                  (`|ExecutionSequence`
                    (:`then_0`
                      ;[1 1 1] Determine class, socket and transform to use
                      (bind (_transform _targetsocket) (`/Game/Mods/CAS/inventory/BP_CAS_inventory_functions.CAS.core.determineEquipTransform` (`local.ItemBeingEquipped`) (`local.ItemSlotBeingEquipped`) (`self.ParentCharacter`)))
                      (set `local.SocketToUse` _targetsocket)
                      (set `local.TransformToUse` _transform)
                      (bind _asbp_attachable (cast `/Game/Mods/CAS/attachables/BP_attachable` (`local.ItemBeingEquipped`)))
                      (bind _targetsocket_2 (`/Game/Mods/CAS/attachables/BP_attachable.TargetSocket` _asbp_attachable))
                      (if (!= _targetsocket_2 "None")
                        (set `local.SocketToUse` _targetsocket_2))
                      (`/Game/Systems/BP_MacroGlobal.IsValid+Branch` (`/Game/Mods/CAS/attachables/BP_attachable.MeshToAttach` _asbp_attachable) true
                        (:`False or Invalid`
                          (bind _isfemale (`/Game/Mods/CAS/inventory/BP_CAS_inventory_functions.CAS.char.getGender` (`self.ParentCharacter`)))
                          (bind _actortoattachfemale (`/Game/Mods/CAS/attachables/BP_attachable.ActorToAttachFemale` _asbp_attachable))
                          (if (and _isfemale (`KismetSystemLibrary.IsValidClass` _actortoattachfemale))
                            (set `local.AttachingActorClass` _actortoattachfemale)
                            (else
                              (set `local.AttachingActorClass` (`/Game/Mods/CAS/attachables/BP_attachable.ActorToAttachMale` _asbp_attachable)))))))
                    (:`then_1`
                      ;[1 1 1] Spawn Attaching Actor, tag it and attach it to the character
                      (bind _worldcomponenttransform (`CharacterFunctionLibrary.GetWorldComponentTransform` (`Character.Mesh` (`self.ParentCharacter`))))
                      (bind _returnvalue (`|SpawnActorFromClass` (`local.AttachingActorClass`) _worldcomponenttransform "Undefined" "OverrideRootScale"))
                      (bind _asbp_attaching_actor (cast `/Game/Mods/CAS/attachables/BP_attaching_actor` _returnvalue))
                      (bind _output_get (set `local.AttachingActor` _asbp_attaching_actor))
                      (set `/Game/Mods/CAS/attachables/BP_attaching_actor.AdditionalMeshTransform` (`local.TransformToUse`) _output_get)
                      (`Actor.K2_AttachToComponent` (`local.AttachingActor`) (`Character.Mesh` (`self.ParentCharacter`)) (`local.SocketToUse`) "SnapToTarget" "SnapToTarget" "SnapToTarget" true)
                      (bind _tag_2 (`/Game/Mods/CAS/inventory/BP_CAS_inventory_functions.CAS.gameItem.generateTag` (`local.ItemBeingEquipped`)))
                      (`KismetArrayLibrary.Array_Add` (`Actor.Tags` (`local.AttachingActor`)) (`KismetStringLibrary.Conv_StringToName` _tag_2)))
                    (:`then_2`
                      ;[1 1 1] Set the appropriate static or skeletal mesh
                      (bind _asbp_attachable_2 (cast `/Game/Mods/CAS/attachables/BP_attachable` (`local.ItemBeingEquipped`))
                        (:`then`
                          (bind _meshtoattach (`/Game/Mods/CAS/attachables/BP_attachable.MeshToAttach` _asbp_attachable_2))
                          (`/Game/Systems/BP_MacroGlobal.IsValid+Branch` _meshtoattach true
                            (:`True`
                              (set `/Game/Mods/CAS/attachables/BP_attaching_actor.StaticMesh` _meshtoattach _attachingactor_2))
                            (:`False or Invalid`
                              (set `/Game/Mods/CAS/attachables/BP_attaching_actor.SkeletalMesh` (`SkinnedMeshComponent.SkeletalMesh` (`/Game/Mods/CAS/attachables/BP_attaching_actor.SkeletalMeshComp` (`local.AttachingActor`))) _attachingactor_2))))
                        (:`CastFailed`
                          (bind (_staticmesh _skeletalmesh) (`/Game/Mods/CAS/inventory/BP_CAS_inventory_functions.CAS.core.findMeshForItem` (`local.ItemBeingEquipped`) (`self.ParentCharacter`)))
                          (`/Game/Systems/BP_MacroGlobal.IsValid+Branch` _staticmesh true
                            (:`True`
                              (set `/Game/Mods/CAS/attachables/BP_attaching_actor.StaticMesh` _staticmesh _attachingactor))
                            (:`False or Invalid`
                              (set `/Game/Mods/CAS/attachables/BP_attaching_actor.SkeletalMesh` _skeletalmesh _attachingactor))))))
                    (:`then_3`
                      ;[1 1 1] Configure physics on the attachment, if needed
                      (bind _settings (`/Game/Mods/CAS/inventory/BP_CAS_inventory_functions.CAS.core.determinePhysicsSettings` (`local.ItemBeingEquipped`) (`local.ItemSlotBeingEquipped`)))
                      (set `/Game/Mods/CAS/attachables/BP_attaching_actor.PhysicsSettings` _settings (`local.AttachingActor`)))
                    (:`then_4`
                      ;[1 1 1] Needed for singleplayer where RepNotify does nothing
                      (if (`KismetSystemLibrary.IsServer`)
                        (`/Game/Mods/CAS/attachables/BP_attaching_actor.OnRep_SkeletalMesh` (`local.AttachingActor`)))))))
              (:`then_3`
                ;[1 1 1] Apply buffs
                (bind _asbp_cas_buff_provider (cast `/Game/Mods/CAS/buffs/BP_CAS_buff_provider` (`local.ItemBeingEquipped`)))
                (bind _buffs (`/Game/Mods/CAS/buffs/BP_CAS_buff_provider.getBuffsToApply` _asbp_cas_buff_provider))
                (for _array_element _buffs
                  (`/Game/Systems/Buffs/00_BP_AC_BuffSystem.AddBuff` (`KismetArrayLibrary.Array_Get` (`Actor.K2_GetComponentsByClass` (`self.ParentCharacter`) "/Game/Systems/Buffs/00_BP_AC_BuffSystem.00_BP_AC_BuffSystem_C")) _array_element _parentcharacter 0 (`/Game/Characters/FuncomFunctionLibrary.GetControllerFromActor` _parentcharacter))))
              (:`then_4`
                ;[1 1 1] Update the CAS.Inventory
                (if (not (`local.ItemIsAlreadyInSlot`))
                  (`/Game/Mods/CAS/inventory/BP_CAS_inventory_functions.CAS.inventory.setItem` (`self.CAS.Inventory`) (`local.ItemSlotBeingEquipped`) (`local.ItemBeingEquipped`))
                  (bind _returnvalue_2 (`ConanCharacter.GetActorPersistenceComponent` (`self.ParentCharacter`)))
                  (`/Game/Systems/BP_MacroGlobal.IsValid+Branch` _returnvalue_2 true
                    (:`True`
                      (`PersistenceComponent.SetDirty` _returnvalue_2 true 5.0)))))
              (:`then_5`
                ;[1 1 1] Fire event
                (`self.DispatchEventItemEquipped` (`local.ItemBeingEquipped`) (`local.ItemSlotBeingEquipped`))
                (return true)))))))
    (else
      (`self.PrintDebug` "Aborting TryEquipItem: called by client!"))))

(fn `CAS.TryEquipItemOnThrall`
  (params (Item :type "GameItem Object Reference") (SlotName :type String) (TargetCharacter :type "/Game/Characters/BaseBPChar Object Reference"))
  (returns (success :type Boolean))
  (if (`KismetSystemLibrary.IsServer`)
    (bind _success (`self.CAS.TryEquipItem` (`Actor.GetComponentByClass` TargetCharacter "BP_CAS_player_comp_C") Item SlotName))
    (return _success)
    (else
      (bind _uniqueid (`/Game/Mods/CAS/inventory/BP_CAS_inventory_functions.CAS.gameitem.generateUID` Item))
      (`self.EventTryEquipItemOnThrall` SlotName _uniqueid TargetCharacter)
      (return true))))

(fn `CAS.TryUnequipItem`
  (params (`CAS.SlotName` :type String))
  (returns (UnequipSuccess :type Boolean))
  (locals (SlotName :type String) (ItemBeingUnequipped :type "GameItem Object Reference") (CASItemBeingUnequipped :type "/Game/Mods/CAS/inventory/CASInventoryItem Structure"))
  (set `local.SlotName` `CAS.SlotName`)
  (if (`KismetSystemLibrary.IsServer`)
    (`self.PrintDebug` "TryUnequipItem" (`KismetSystemLibrary.GetDisplayName` (`self.ParentCharacter`)) (`local.SlotName`)
      (:`execOut`
        (`|ExecutionSequence`
          (:`then_0`
            ;[1 1 1] Remove item from CAS inventory
            (bind _previousitem (`/Game/Mods/CAS/inventory/BP_CAS_inventory_functions.CAS.inventory.removeItem` (`self.CAS.Inventory`) (`local.SlotName`)))
            (bind _output_get (set `local.CASItemBeingUnequipped` _previousitem))
            (bind _item (`/Game/Mods/CAS/inventory/BP_CAS_inventory_functions.CAS.item.resolveOnChar` _output_get (`self.ParentCharacter`)))
            (set `local.ItemBeingUnequipped` _item))
          (:`then_1`
            ;[1 1 1] Remove item visual
            (bind _matchedactors (`/Game/Mods/CAS/inventory/BP_CAS_inventory_functions.CAS.char.findAttachedActorsByTag` (`self.ParentCharacter`) (`KismetStringLibrary.Concat_StrStr` "CAS.attached." (`.GameItemID_11_07FD5B0E4AB07E5A4472A18811FFE6D4` (break `/Game/Mods/CAS/inventory/CASInventoryItem` (`local.CASItemBeingUnequipped`))))))
            (for _array_element _matchedactors
              (`Actor.K2_DestroyActor` _array_element)))
          (:`then_2`
            ;[1 1 1] Stop any buffs
            (bind _asbp_cas_buff_provider (cast `/Game/Mods/CAS/buffs/BP_CAS_buff_provider` (`local.ItemBeingUnequipped`)))
            (bind _buffs (`/Game/Mods/CAS/buffs/BP_CAS_buff_provider.getBuffsToApply` _asbp_cas_buff_provider))
            (for _array_element_2 _buffs
              (`/Game/Systems/Buffs/00_BP_AC_BuffSystem.RemoveBuff` (`KismetArrayLibrary.Array_Get` (`Actor.K2_GetComponentsByClass` (`self.ParentCharacter`) "/Game/Systems/Buffs/00_BP_AC_BuffSystem.00_BP_AC_BuffSystem_C")) _array_element_2)))
          (:`then_3`
            ;[1 1 1] Flag dirty for persistence
            (bind _returnvalue (`ConanCharacter.GetActorPersistenceComponent` (`self.ParentCharacter`)))
            (`/Game/Systems/BP_MacroGlobal.IsValid+Branch` _returnvalue true
              (:`True`
                (`PersistenceComponent.SetDirty` _returnvalue true 5.0))))
          (:`then_4`
            ;[1 1 1] Fire event
            (`self.DispatchEventItemUnequipped` (`local.ItemBeingUnequipped`) (`local.SlotName`))
            (return true)))))
    (else
      (`self.PrintDebug` "Aborting TryUnequipItem: called by client!"))))

(fn `CAS.TryUnequipItemOnThrall`
  (params (SlotName :type String) (TargetCharacter :type "/Game/Characters/BaseBPChar Object Reference"))
  (returns (success :type Boolean))
  (if (`KismetSystemLibrary.IsServer`)
    (bind _unequipsuccess (`self.CAS.TryUnequipItem` (`Actor.GetComponentByClass` TargetCharacter "BP_CAS_player_comp_C") SlotName))
    (return _unequipsuccess)
    (else
      (`self.EventTryUnequipItemOnThrall` SlotName TargetCharacter)
      (return true))))